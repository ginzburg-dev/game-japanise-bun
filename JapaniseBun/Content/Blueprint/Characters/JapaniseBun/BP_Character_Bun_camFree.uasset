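; Player-controlled Bun character with a flipbook sprite, Enhanced Input movement and double jump.
; Mouse X accumulates a yaw that steers movement input, while the code that would rotate the actor or spring arm is disconnected.
; Each tick derives an animation state from velocity, selects its flipbook and flips facing along world X.
; Overlapping a BP_Dot on DangerCheck sets sprite facing and triggers a timed Jam stun that suspends animation and facing updates.
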(event OnComponentBeginOverlap(DangerCheck)
  (params (OverlappedComponent :type Primitive%20Component%20Object%20Reference) (OtherActor :type Actor%20Object%20Reference) (OtherComp :type Primitive%20Component%20Object%20Reference) (OtherBodyIndex :type Integer) (bFromSweep :type Boolean) (SweepResult :type Hit%20Result%20Structure%20%28by%20ref%29))
  (bind _direction (Variables|Default|GetDirection))
  (bind _returnvalue (< _direction 0.0))
  (bind _asbp_dot (Utilities|Casting|CastToBP_Dot OtherActor))
  (bind _x (CallFunction|DangerDirection _asbp_dot))
  (if (and (> _x 0.0) _returnvalue)
    (Transformation|SetRelativeRotation (Variables|Default|GetSprite) "0.000000,180.000000,0.000000" false false :!label _label)
    (elif (and (not (> _x 0.0)) (not _returnvalue))
      (goto _label)
      (elif (and (not (> _x 0.0)) _returnvalue)
        (goto _label)
        (else
          _))))
  (CallFunction|ReciveAttack "NewEnumerator1")
  (CallFunction|UpdateAnimation))

(event Custom|UpdateAnimation
  (bind _returnvalue (Transformation|GetVelocity))
  (bind _returnvalue_2 (Math|Float|Absolute(Float) (.z _returnvalue)))
  (bind _returnvalue_3 (> _returnvalue_2 0.0))
  (if (not (Variables|Default|GetisStunned))
    (if (and (> (Math|Vector|VectorLength (Transformation|GetVelocity)) 0.0) (AI|Components|NavMovement|IsMovingonGround (Variables|Character|GetCharacterMovement)))
      (Variables|Default|SetAnimationState "NewEnumerator4")
      (Variables|Default|SetisJump false)
      (elif (and _returnvalue_3 (not (Variables|Default|GetisJump)))
        (Variables|Default|SetAnimationState "NewEnumerator2")
        (Utilities|FlowControl|Delay 0.1)
        (Variables|Default|SetAnimationState "NewEnumerator1")
        (Variables|Default|SetisJump true)
        (elif (and (Variables|Default|GetisJump) (not _returnvalue_3))
          (Variables|Default|SetAnimationState "NewEnumerator3")
          (Utilities|FlowControl|Delay 0.1)
          (Variables|Default|SetAnimationState "NewEnumerator0")
          (Variables|Default|SetisJump false)
          (elif (and _returnvalue_3 (Variables|Default|GetisJump))
            (Variables|Default|SetAnimationState "NewEnumerator1")
            (Variables|Default|SetisJump true)
            (else
              (Variables|Default|SetAnimationState "NewEnumerator0")
              (Variables|Default|SetisJump false))))))))

(event Custom|SpriteShake
  (bind _returnvalue (Math|Random|RandomFloatinRange -1e+01 1e+01))
  (if (Variables|Default|GetisShaking)
    (Transformation|SetRelativeLocation (Variables|Default|GetSprite) (+ "" (Math|Vector|MakeVector _returnvalue _returnvalue _returnvalue)) false false)))

(event Custom|CleanShake
  (Variables|Default|SetisShaking false)
  (Transformation|SetRelativeLocation (Variables|Default|GetSprite) (Variables|Default|GetSpritePos) false false))

(event Custom|Lounch
  (Physics|AddImpulse (Variables|Character|GetCharacterMovement) (Math|Vector|MakeVector 0.0 0.0 (Variables|Default|GetImpulse%20Z)) false))

(event Input|EnhancedActionEvents|EnhancedInputActionAI_Move
  (params (ActionValue :type Vector%202D%20Structure) (ElapsedSeconds :type Float%20%28double-precision%29) (TriggeredSeconds :type Float%20%28double-precision%29) (InputAction :type Input%20Action%20Object%20Reference :default "/Game/Blueprint/Characters/JapaniseBun/Actions/AI_Move.AI_Move"))
  (bind (_x _y) (Math|Vector2D|BreakVector2D ActionValue))
  (:Triggered
    (Pawn|Input|AddMovementInput (Math|Vector|RotateVector "1.000000,0.000000,0.000000" (Variables|Default|GetaddRotator)) _x false)
    (Pawn|Input|AddMovementInput (Math|Vector|RotateVector "0.000000,-1.000000,0.000000" (Variables|Default|GetaddRotator)) _y false)
    (CallFunction|UpdateAnimation)))

(event Input|EnhancedActionEvents|EnhancedInputActionAI_Jump
  (params (ActionValue :type Boolean) (ElapsedSeconds :type Float%20%28double-precision%29) (TriggeredSeconds :type Float%20%28double-precision%29) (InputAction :type Input%20Action%20Object%20Reference :default "/Game/Blueprint/Characters/JapaniseBun/Actions/AI_Jump.AI_Jump"))
  (:Started
    (Character|Jump)
    (CallFunction|UpdateAnimation))
  (:Canceled
    (Character|StopJumping :!label _label))
  (:Completed
    (goto _label)))

(event Input|EnhancedActionEvents|EnhancedInputActionAI_MouseMove
  (params (ActionValue :type Vector%202D%20Structure) (ElapsedSeconds :type Float%20%28double-precision%29) (TriggeredSeconds :type Float%20%28double-precision%29) (InputAction :type Input%20Action%20Object%20Reference :default "/Game/Blueprint/Characters/JapaniseBun/Actions/AI_MouseMove.AI_MouseMove"))
  (:Triggered
    (Variables|Default|SetinputMouse ActionValue :!label _label))
  (:Started
    (goto _label))
  (:Ongoing
    (goto _label)))

(event EventBeginPlay
  (|CallParentFunction)
  (bind _asplayer_controller (Utilities|Casting|CastToPlayerController (Game|GetPlayerController 0)))
  (Input|AddMappingContext (PlayerController|LocalPlayerSubsystems|GetEnhancedInputLocalPlayerSubsystem _asplayer_controller) "/Game/Input/IMC_Bun.IMC_Bun" 0 "(bIgnoreAllPressedKeysUntilRelease=True,bForceImmediately=False)")
  (Variables|Default|SetJumpMaxCount 2)
  (Variables|Default|SetSpritePos (Variables|/Script/Engine.SceneComponent|GetRelativeLocation (Variables|Default|GetSprite))))

(event Collision|EventActorBeginOverlap
  (params (OtherActor :type Actor%20Object%20Reference))
  (|CallParentFunction OtherActor) ; This node is disabled and will not be called.\nDrag off pins to build functionality.
)

(event EventTick
  (params (DeltaSeconds :type Float%20%28single-precision%29))
  (|CallParentFunction DeltaSeconds)
  (CallFunction|UpdateAnimation)
  (bind _returnvalue (CallFunction|SetAnimationState))
  (Sprite|SetFlipbook (Variables|Default|GetSprite) _returnvalue)
  (CallFunction|MouseRotate DeltaSeconds (Variables|Default|GetinputMouse))
  (CallFunction|Rotate))

(fn ConstructionScript
  (|CallParentFunction))

(fn SetAnimationState
  (return (Utilities|Select :Index (Variables|Default|GetAnimationState) :NewEnumerator0 (Variables|Default|GetIdle%20Flipbook) :NewEnumerator1 (Variables|Default|GetJump%20Flipbook) :NewEnumerator2 (Variables|Default|GetinJump) :NewEnumerator3 (Variables|Default|GetoutJump) :NewEnumerator4 (Variables|Default|GetWalk) :NewEnumerator5 0 :NewEnumerator6 (Variables|Default|GetstunJam) :NewEnumerator7 (Variables|Default|GetstunStandard) :NewEnumerator8 0 :NewEnumerator9 0 :NewEnumerator10 0 :NewEnumerator11 0)))

(fn Rotate
  (bind _returnvalue (Transformation|GetVelocity))
  (if (not (Variables|Default|GetisStunned))
    (Transformation|SetWorldRotation (Variables|Default|GetSprite) "0, 0, 0" false false)
    (if (> (.x _returnvalue) 0.0)
      (Transformation|SetActorRotation "0, 0, 0")
      (Variables|Default|SetActorRot "0, 0, 0")
      (Variables|Default|SetDirection 1.0)
      (elif (< (.x _returnvalue) 0.0)
        (Transformation|SetActorRotation "0.000000,180.000000,0.000000")
        (Variables|Default|SetActorRot "0.000000,180.000000,0.000000")
        (Variables|Default|SetDirection -1.0)
        (else
          (Transformation|SetActorRotation (Variables|Default|GetActorRot)))))))

(fn ReciveAttack
  (params (StunType :type E_Stun%20Enum :default "NewEnumerator0"))
  (Variables|Default|SetisStunned true)
  (Variables|Default|SetAnimationState (Utilities|Select :Index StunType :NewEnumerator0 "NewEnumerator7" :NewEnumerator1 "NewEnumerator6"))
  (Utilities|Time|SetTimerbyEvent (EventDispatchers|CreateEvent :!event ClearStun) (Variables|Default|GetStunLength))
  (return))

(fn ClearStun
  (Variables|Default|SetisStunned false)
  (Variables|Default|SetAnimationState "NewEnumerator0"))

(fn DangerDirection
  (params (TargetHit :type Actor%20Object%20Reference))
  (bind _asbp_dot (Utilities|Casting|CastToBP_Dot TargetHit))
  (return (.x (- (Transformation|GetActorLocation (Variables|/Game/Blueprint/Characters/Donut/BP_Dot.BP_Dot_C|GetEnemy _asbp_dot)) (Transformation|GetActorLocation)))))

(fn MouseRotate
  (params (DeltaSeconds :type Float%20%28double-precision%29) (MouseInputXY :type Vector%202D%20Structure))
  (Variables|Default|SetaddRotator (Math|Rotator|MakeRotator 0.0 0.0 (+ (* DeltaSeconds (.x MouseInputXY) (Variables|Default|GetmouseSpeed)) (.yaw (Variables|Default|GetaddRotator))))))