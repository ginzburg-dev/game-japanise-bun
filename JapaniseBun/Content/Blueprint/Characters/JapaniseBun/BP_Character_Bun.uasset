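; Player-controlled bun character with flipbook sprites, Enhanced Input movement, double jump, wall slide and jump, and energy-limited power walk.
; Tick updates energy, camera effects and an animation state that selects the flipbook, with line traces detecting walls.
; Power jump blends upward impulse with a direction computed from the nearest unobstructed living BP_Donut.
; BP_Dot overlaps below a speed threshold damage and stun; death zooms the camera and opens the kitchen map.
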(event OnComponentBeginOverlap(DangerCheck)
  (params (OverlappedComponent :type Primitive%20Component%20Object%20Reference) (OtherActor :type Actor%20Object%20Reference) (OtherComp :type Primitive%20Component%20Object%20Reference) (OtherBodyIndex :type Integer) (bFromSweep :type Boolean) (SweepResult :type Hit%20Result%20Structure%20%28by%20ref%29))
  (bind _direction (Variables|Default|GetDirection))
  (bind _returnvalue (< _direction 0.0))
  (if (not (>= (Math|Vector|VectorLength (Transformation|GetVelocity)) (Variables|Default|GetReciveAttackMinZVelocity)))
    (bind _asbp_dot (Utilities|Casting|CastToBP_Dot OtherActor))
    (if (not (Variables|Default|GetisDead))
      (bind _x (CallFunction|DangerDirection _asbp_dot))
      (if (and (> _x 0.0) _returnvalue)
        (Transformation|SetRelativeRotation (Variables|Default|GetSprite) "0.000000,180.000000,0.000000" false false :!label _label)
        (elif (and (not (> _x 0.0)) (not _returnvalue))
          (goto _label)
          (elif (and (not (> _x 0.0)) _returnvalue)
            (goto _label)
            (else
              _))))
      (CallFunction|ReciveAttack "NewEnumerator1" (Variables|/Game/Blueprint/Characters/Donut/BP_Dot.BP_Dot_C|GetDamage _asbp_dot))
      (CallFunction|UpdateAnimation))))

(event Custom|UpdateAnimation
  (bind _returnvalue (Transformation|GetVelocity))
  (bind _returnvalue_2 (Math|Float|Absolute(Float) (.z _returnvalue)))
  (bind _returnvalue_3 (> _returnvalue_2 0.0))
  (CallFunction|EnergyRaise)
  (CallFunction|CameraMBlur)
  (CallFunction|DeadCamera)
  (if (<= (Variables|Default|GetHealth) 0.0)
    (Utilities|FlowControl|DoOnce false
      (:Completed
        (CallFunction|Dead)))
    (else
      (bind _isslidewall (CallFunction|IsWallSliding))
      (Variables|Default|SetisSladeWall _isslidewall)
      (if (Variables|Default|GetisStunned)
        (CallFunction|SpriteShake)
        (Utilities|Time|SetTimerbyEvent (delegate Custom|CleanShake) 0.05 true)
        (elif (and (> (Math|Vector|VectorLength (Transformation|GetVelocity)) 0.0) (AI|Components|NavMovement|IsMovingonGround (Variables|Character|GetCharacterMovement)))
          (Variables|Default|SetAnimationState "NewEnumerator4")
          (Variables|Default|SetisJump false)
          (elif (and _returnvalue_3 (not (Variables|Default|GetisJump)))
            (if (Variables|Default|GetisSladeWall)
              _
              (else
                (Variables|Default|SetAnimationState "NewEnumerator2")
                (Utilities|FlowControl|Delay 0.1)))
            (Variables|Default|SetAnimationState "NewEnumerator1")
            (Variables|Default|SetisJump true)
            (elif (and (Variables|Default|GetisJump) (not _returnvalue_3))
              (if (Variables|Default|GetisSladeWall)
                _
                (else
                  (Variables|Default|SetAnimationState "NewEnumerator3")
                  (Utilities|FlowControl|Delay 0.1)))
              (Variables|Default|SetAnimationState "NewEnumerator0")
              (Variables|Default|SetisJump false)
              (elif (and _returnvalue_3 (Variables|Default|GetisJump))
                (Variables|Default|SetAnimationState "NewEnumerator1")
                (Variables|Default|SetisJump true)
                (else
                  (Variables|Default|SetAnimationState "NewEnumerator0")
                  (Variables|Default|SetisJump false))))))))))

(event Custom|SpriteShake
  (bind _camerashakeintensity (Variables|Default|GetCameraShakeIntensity))
  (bind _returnvalue (* _camerashakeintensity -1.0))
  (bind _returnvalue_2 (Math|Random|RandomFloatinRange _returnvalue _camerashakeintensity))
  (Transformation|SetRelativeLocation (Variables|Default|GetSprite) (+ "" (Math|Vector|MakeVector _returnvalue_2 _returnvalue_2 _returnvalue_2)) false false))

(event Custom|CleanShake
  (Variables|Default|SetisShaking false)
  (Transformation|SetRelativeLocation (Variables|Default|GetSprite) (Variables|Default|GetSpritePos) false false))

(event Custom|Lounch
  (bind _impulse_z (Variables|Default|GetImpulse%20Z))
  (bind _returnvalue (Math|Vector|MakeVector 0.0 0.0 _impulse_z))
  (if (> (Variables|Default|GetAutoTarget) 0.0)
    (bind (_result_actor _result) (CallFunction|GetNearEnemyPosition (Variables|Default|GetEnemyArray)))
    (if _result
      (Variables|Default|SetPowerJumpVector (Math|Vector|Lerp(Vector) _returnvalue (* (Math|Vector|Normalize (- (Transformation|GetActorLocation) (Transformation|GetActorLocation _result_actor))) (Math|Vector|MakeVector _impulse_z _impulse_z _impulse_z)) (Variables|Default|GetAutoTarget)))
      (else
        (Variables|Default|SetPowerJumpVector _returnvalue :!label _label)))
    (else
      (goto _label)))
  (Physics|AddImpulse (Variables|Character|GetCharacterMovement) (Variables|Default|GetPowerJumpVector) false))

(event Custom|CleanDead
  (Variables|Default|SetAnimationState "NewEnumerator10")
  (bind _returnvalue (CallFunction|SetAnimationState))
  (Sprite|SetFlipbook (Variables|Default|GetSprite) _returnvalue)
  (Input|RemoveMappingContext (PlayerController|LocalPlayerSubsystems|GetEnhancedInputLocalPlayerSubsystem (Game|GetPlayerController 0)) "/Game/Input/IMC_Bun.IMC_Bun" "(bIgnoreAllPressedKeysUntilRelease=True,bForceImmediately=False)")
  (Utilities|FlowControl|Delay 1.0)
  (Game|OpenLevel(byName) "MAP_KITCHEN_0000"))

(event Custom|NegativeLounch
  (bind _negativelounchmult (Variables|Default|GetNegativeLounchMult))
  (Variables|Default|SetCurrentNegativeLounchVector (* (Transformation|GetVelocity) (Math|Vector|MakeVector _negativelounchmult _negativelounchmult _negativelounchmult)))
  (Variables|/Script/Engine.MovementComponent|SetVelocity (Variables|Character|GetCharacterMovement) "0, 0, 0")
  (Physics|AddImpulse (Variables|Character|GetCharacterMovement) (Variables|Default|GetCurrentNegativeLounchVector) false))

(event Custom|CameraMBlur
  (Variables|/Script/Engine.CameraComponent|SetPostProcessSettings (Variables|Default|GetCamera) (Utilities|Struct|MakePostProcessSettings (Math|Float|Lerp 0.0 (Variables|Default|GetMaxMotionBlur) (/ (Math|Float|Absolute(Float) (.x (Transformation|GetVelocity))) (Variables|Default|GetPowerWalkSpeed))))))

(event Input|EnhancedActionEvents|EnhancedInputActionAI_Move
  (params (ActionValue :type Vector%202D%20Structure) (ElapsedSeconds :type Float%20%28double-precision%29) (TriggeredSeconds :type Float%20%28double-precision%29) (InputAction :type Input%20Action%20Object%20Reference :default "/Game/Blueprint/Characters/JapaniseBun/Actions/AI_Move.AI_Move"))
  (bind (_x _y) (Math|Vector2D|BreakVector2D ActionValue))
  (:Triggered
    (Pawn|Input|AddMovementInput "1.000000,0.000000,0.000000" _x false)
    (Pawn|Input|AddMovementInput "0.000000,-1.000000,0.000000" _y false)))

(event Input|EnhancedActionEvents|EnhancedInputActionAI_Jump
  (params (ActionValue :type Boolean) (ElapsedSeconds :type Float%20%28double-precision%29) (TriggeredSeconds :type Float%20%28double-precision%29) (InputAction :type Input%20Action%20Object%20Reference :default "/Game/Blueprint/Characters/JapaniseBun/Actions/AI_Jump.AI_Jump"))
  (bind _walllounchforce (Variables|Default|GetWallLounchForce))
  (:Started
    (if (Variables|Default|GetisSladeWall)
      (Variables|Default|SetJumpMaxCount 1)
      (Character|LaunchCharacter (Class|CharacterMovementComponent|GetCharacterOwner (Variables|Character|GetCharacterMovement)) (+ (* (Variables|Default|GetWallHitNormal) (Math|Vector|MakeVector _walllounchforce 0.0 0.0)) (Math|Vector|MakeVector 0.0 0.0 (* _walllounchforce 2.0))) false false)
      (else
        (Variables|Default|SetJumpMaxCount 2)
        (Character|Jump))))
  (:Canceled
    (Character|StopJumping :!label _label))
  (:Completed
    (goto _label)))

(event Input|EnhancedActionEvents|EnhancedInputActionAI_MouseMove
  (params (ActionValue :type Vector%202D%20Structure) (ElapsedSeconds :type Float%20%28double-precision%29) (TriggeredSeconds :type Float%20%28double-precision%29) (InputAction :type Input%20Action%20Object%20Reference :default "/Game/Blueprint/Characters/JapaniseBun/Actions/AI_MouseMove.AI_MouseMove"))
  (:Triggered
    (Variables|Default|SetinputMouse ActionValue :!label _label))
  (:Started
    (goto _label))
  (:Ongoing
    (goto _label)))

(event Input|EnhancedActionEvents|EnhancedInputActionAI_PowerWalk
  (params (ActionValue :type Boolean) (ElapsedSeconds :type Float%20%28double-precision%29) (TriggeredSeconds :type Float%20%28double-precision%29) (InputAction :type Input%20Action%20Object%20Reference :default "/Game/Blueprint/Characters/JapaniseBun/Actions/AI_PowerWalk.AI_PowerWalk"))
  (bind _charactermovement (Variables|Character|GetCharacterMovement))
  (bind _walkspeed (Variables|Default|GetWalkSpeed))
  (:Triggered
    (if (> (Variables|Default|GetEnergy) 0.0)
      (Variables|Default|SetisPower true)
      (CallFunction|EnergyReduce)
      (Variables|/Script/Engine.CharacterMovementComponent|SetMaxWalkSpeed _charactermovement (Variables|Default|GetPowerWalkSpeed))
      (else
        (Variables|Default|SetisPower false)
        (Variables|/Script/Engine.CharacterMovementComponent|SetMaxWalkSpeed _charactermovement _walkspeed))))
  (:Canceled
    (Variables|Default|SetisPower false :!label _label)
    (Variables|/Script/Engine.CharacterMovementComponent|SetMaxWalkSpeed _charactermovement _walkspeed))
  (:Completed
    (goto _label)))

(event Input|EnhancedActionEvents|EnhancedInputActionAI_PowerDownJump
  (params (ActionValue :type Boolean) (ElapsedSeconds :type Float%20%28double-precision%29) (TriggeredSeconds :type Float%20%28double-precision%29) (InputAction :type Input%20Action%20Object%20Reference :default "/Game/Blueprint/Characters/JapaniseBun/Actions/AI_PowerDownJump.AI_PowerDownJump"))
  (:Started
    (CallFunction|Lounch)))

(event EventBeginPlay
  (|CallParentFunction)
  (bind _asplayer_controller (Utilities|Casting|CastToPlayerController (Game|GetPlayerController 0)))
  (Input|AddMappingContext (PlayerController|LocalPlayerSubsystems|GetEnhancedInputLocalPlayerSubsystem _asplayer_controller) "/Game/Input/IMC_Bun.IMC_Bun" 0 "(bIgnoreAllPressedKeysUntilRelease=True,bForceImmediately=False)")
  (Variables|Default|SetJumpMaxCount 2)
  (Variables|Default|SetSpritePos (Variables|/Script/Engine.SceneComponent|GetRelativeLocation (Variables|Default|GetSprite)))
  (bind _returnvalue (UserInterface|CreateWidget "/Game/UI/WB_HUD.WB_HUD_C"))
  (bind _output_get (Variables|Default|SetHUDReference _returnvalue))
  (UserInterface|Viewport|AddtoViewport _output_get 0)
  (Variables|/Script/Engine.CharacterMovementComponent|SetMaxWalkSpeed (Variables|Character|GetCharacterMovement) (Variables|Default|GetWalkSpeed))
  (bind _outactors (Actor|GetAllActorsOfClass "/Game/Blueprint/Characters/Donut/BP_Donut.BP_Donut_C"))
  (Variables|Default|SetEnemyArray _outactors))

(event Collision|EventActorBeginOverlap
  (params (OtherActor :type Actor%20Object%20Reference))
  (|CallParentFunction OtherActor) ; This node is disabled and will not be called.\nDrag off pins to build functionality.
)

(event EventTick
  (params (DeltaSeconds :type Float%20%28single-precision%29))
  (|CallParentFunction DeltaSeconds)
  (Variables|Default|SetTime (Utilities|Time|GetGameTimeinSeconds))
  (CallFunction|UpdateAnimation)
  (if (not (Variables|Default|GetisDead))
    (bind _returnvalue (CallFunction|SetAnimationState))
    (Sprite|SetFlipbook (Variables|Default|GetSprite) _returnvalue)
    (CallFunction|MouseRotate DeltaSeconds (Variables|Default|GetinputMouse))
    (CallFunction|Rotate)))

(fn ConstructionScript
  (|CallParentFunction))

(fn SetAnimationState
  (return (Utilities|Select :Index (Variables|Default|GetAnimationState) :NewEnumerator0 (Variables|Default|GetIdle%20Flipbook) :NewEnumerator1 (Variables|Default|GetJump%20Flipbook) :NewEnumerator2 (Variables|Default|GetinJump) :NewEnumerator3 (Variables|Default|GetoutJump) :NewEnumerator4 (Variables|Default|GetWalk) :NewEnumerator5 0 :NewEnumerator6 (Variables|Default|GetstunJam) :NewEnumerator7 (Variables|Default|GetstunStandard) :NewEnumerator8 (Variables|Default|GetDead_fall) :NewEnumerator9 0 :NewEnumerator10 (Variables|Default|GetDead_fall_static) :NewEnumerator11 0)))

(fn Rotate
  (bind _returnvalue (Transformation|GetVelocity))
  (bind _sprite (Variables|Default|GetSprite))
  (if (not (Variables|Default|GetisStunned))
    (Transformation|SetWorldRotation (Variables|Default|GetSprite) "0, 0, 0" false false)
    (if (> (.x _returnvalue) 0.0)
      (Transformation|SetWorldRotation _sprite "0, 0, 0" false false)
      (Variables|Default|SetActorRot "0, 0, 0")
      (Variables|Default|SetDirection 1.0)
      (elif (< (.x _returnvalue) 0.0)
        (Transformation|SetWorldRotation _sprite "0.000000,180.000000,0.000000" false false)
        (Variables|Default|SetActorRot "0.000000,180.000000,0.000000")
        (Variables|Default|SetDirection -1.0)
        (else
          (Transformation|SetWorldRotation _sprite (Variables|Default|GetActorRot) false false))))))

(fn ReciveAttack
  (params (StunType :type E_Stun%20Enum :default "NewEnumerator0") (Damage :type Float%20%28double-precision%29))
  (Variables|Default|SetisStunned true)
  (Variables|Default|SetAnimationState (Utilities|Select :Index StunType :NewEnumerator0 "NewEnumerator7" :NewEnumerator1 "NewEnumerator6"))
  (Variables|Default|SetHealth (- (Variables|Default|GetHealth) Damage))
  (Utilities|Time|SetTimerbyEvent (EventDispatchers|CreateEvent :!event ClearStun) (Variables|Default|GetStunLength))
  (return))

(fn ClearStun
  (Variables|Default|SetisStunned false)
  (if (not (Variables|Default|GetisDead))
    (Variables|Default|SetAnimationState "NewEnumerator0")))

(fn DangerDirection
  (params (TargetHit :type Actor%20Object%20Reference))
  (bind _asbp_dot (Utilities|Casting|CastToBP_Dot TargetHit))
  (return (.x (- (Transformation|GetActorLocation _asbp_dot) (Transformation|GetActorLocation)))))

(fn MouseRotate
  (params (DeltaSeconds :type Float%20%28double-precision%29) (MouseInputXY :type Vector%202D%20Structure))
  (Variables|Default|SetaddRotator (Math|Rotator|MakeRotator 0.0 0.0 (+ (* DeltaSeconds (.x MouseInputXY) (Variables|Default|GetmouseSpeed)) (.yaw (Variables|Default|GetaddRotator))))))

(fn IsWallSliding
  (bind _returnvalue (Transformation|GetActorLocation))
  (bind _slidewalldistance (Variables|Default|GetSlideWallDistance))
  (if (and (AI|Components|NavMovement|IsFalling (Variables|Character|GetCharacterMovement)) (Variables|Default|GetisWallJumpingOn))
    (bind (_outhit _returnvalue_2) (Collision|LineTraceByChannel _returnvalue (+ _returnvalue (* (Math|Vector|MakeVector (Variables|Default|GetDirection) 0.0 0.0) (Math|Vector|MakeVector _slidewalldistance _slidewalldistance _slidewalldistance))) "TraceTypeQuery1" false 0 "None"))
    (bind _output_get (Variables|Default|SetisSladeWall _returnvalue_2))
    (Variables|Default|SetWallHitNormal (.ImpactNormal (Collision|BreakHitResult _outhit)))
    (if _output_get
      (Variables|/Script/Engine.MovementComponent|SetVelocity (Variables|Character|GetCharacterMovement) (Math|Interpolation|VInterptoConstant (Transformation|GetVelocity) "0, 0, 0" (Utilities|Time|GetWorldDeltaSeconds) 2e+03))
      (Development|PrintString (Utilities|String|ToString(Vector) (Transformation|GetVelocity))))
    (return _output_get)))

(fn Dead
  (if (Variables|Default|GetisDead)
    (Variables|Default|SetAnimationState "NewEnumerator10")
    (else
      (Variables|Default|SetAnimationState "NewEnumerator8")
      (Variables|Default|SetisDead true)))
  (bind _returnvalue (CallFunction|SetAnimationState))
  (Sprite|SetFlipbook (Variables|Default|GetSprite) _returnvalue)
  (Utilities|Time|SetTimerbyEvent (EventDispatchers|CreateEvent :!event Custom|CleanDead) 0.2))

(fn DeadCamera
  (bind _springarm (Variables|Default|GetSpringArm))
  (if (Variables|Default|GetisDead)
    (Variables|/Script/Engine.SpringArmComponent|SetTargetArmLength _springarm (Math|Interpolation|FInterptoConstant (Variables|/Script/Engine.SpringArmComponent|GetTargetArmLength _springarm) (Variables|Default|GetDeadCameraLength) (Utilities|Time|GetWorldDeltaSeconds) 1e+02))))

(fn GetNearEnemy
  (bind _outactors (Actor|GetAllActorsOfClass "/Game/Blueprint/Characters/Donut/BP_Donut.BP_Donut_C"))
  (return (.ReturnValue (Actor|FindNearestActor (Transformation|GetActorLocation) _outactors))))

(fn GetNearEnemyPosition
  (params (Array :type Array%20of%20Actor%20Object%20References))
  (bind _returnvalue (Transformation|GetActorLocation))
  (Variables|Default|SetCurrentNearEnemy 0)
  (Variables|Default|SetCurrentNearDistance (Variables|Default|GetMaxNaerEnemyDistance))
  (if (Utilities|Array|IsNotEmpty Array)
    (for _array_element Array
      (bind _asbp_donut (Utilities|Casting|CastToBP_Donut _array_element))
      (if (not (Variables|/Game/Blueprint/Characters/Donut/BP_Donut.BP_Donut_C|GetisDead _asbp_donut))
        (bind _returnvalue_2 (Collision|LineTraceForObjects _returnvalue (Transformation|GetActorLocation _array_element) (Variables|Default|GetObject%20Types) false 0 "None"))
        (if (not _returnvalue_2)
          (if (< (Math|Vector|Distance(Vector) _returnvalue (Transformation|GetActorLocation _array_element)) (Variables|Default|GetCurrentNearDistance))
            (Variables|Default|SetCurrentNearDistance (Math|Vector|Distance(Vector) _returnvalue (Transformation|GetActorLocation _array_element)))
            (Variables|Default|SetCurrentNearEnemy _array_element))))))
  (return (Variables|Default|GetCurrentNearEnemy) (Utilities|IsValid (Variables|Default|GetCurrentNearEnemy))))

(fn EnergyReduce
  (if (Variables|Default|GetisPower)
    (Variables|Default|SetEnergy (Math|Interpolation|FInterptoConstant (Variables|Default|GetEnergy) 0.0 (Utilities|Time|GetWorldDeltaSeconds) (Variables|Default|GetEnergyReduceSpeed)))
    (return)))

(fn EnergyRaise
  (if (not (Variables|Default|GetisPower))
    (Variables|Default|SetEnergy (Math|Interpolation|FInterptoConstant (Variables|Default|GetEnergy) 1.0 (Utilities|Time|GetWorldDeltaSeconds) (Variables|Default|GetEnergyRaiseSpeed)))
    (return)))