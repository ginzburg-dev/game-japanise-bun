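; Donut enemy character with Paper2D flipbooks that throws BP_Dot projectiles at the Bun player and can be killed by a stomp.
; Tick flips the sprite by velocity, picks the animation state and detects whether Bun is in the near or far zone.
; OnAttacking fires randomized bursts while stationary, with impulses shaped by that zone and Bun's side.
; A fast-falling Bun entering DangerCheck triggers a random death, stopping AI and collision, and gets launched.
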(event OnComponentBeginOverlap(DangerCheck)
  (params (OverlappedComponent :type Primitive%20Component%20Object%20Reference) (OtherActor :type Actor%20Object%20Reference) (OtherComp :type Primitive%20Component%20Object%20Reference) (OtherBodyIndex :type Integer) (bFromSweep :type Boolean) (SweepResult :type Hit%20Result%20Structure%20%28by%20ref%29))
  (bind _asbp_character_bun (Utilities|Casting|CastToBP_Character_Bun OtherActor))
  (if (and (< (.z (Transformation|GetVelocity _asbp_character_bun)) 0.0) (>= (Math|Vector|VectorLength (Math|Vector|MakeVector (.x (Transformation|GetVelocity _asbp_character_bun)) (.y (Transformation|GetVelocity _asbp_character_bun)) (.z (Transformation|GetVelocity _asbp_character_bun)))) (Variables|Default|GetDangerVelocityLevel)))
    (bind _output_get (Variables|Default|SetDeadType (.OutItem (Utilities|Array|Random (Utilities|Array|MakeArray "NewEnumerator0" "NewEnumerator1")))))
    (CallFunction|Dead _output_get)
    (Default|NegativeLounch _asbp_character_bun)))

(event Custom|OnAttacking
  (if (not (Variables|Default|GetisDead))
    (if (Variables|Default|GetisAttacking)
      _
      (else
        (Variables|Default|SetAttackVarCounter 0)
        (Variables|Default|SetAttackCounter (Math|Random|RandomIntegerinRange (Variables|Default|GetMinAttackCount) (Variables|Default|GetMaxAttackCount)))
        (Variables|Default|SetAnimationState "NewEnumerator5")))
    (if (< (Variables|Default|GetAttackVarCounter) (Variables|Default|GetAttackCounter)) :!label _label
      (if (Variables|Default|GetisAttacking)
        (Utilities|FlowControl|Delay (Math|Random|RandomFloatinRange (Variables|Default|GetMinAttackDelay) (Variables|Default|GetMaxAttackDelay))))
      (Variables|Default|SetisAttacking true)
      (bind _result (Math|Integer|IncrementInt (Variables|Default|GetAttackVarCounter))
        (:%20%20
          (Variables|Default|SetAttackVarCounter _result)
          (if (<= (Math|Vector|VectorLength (Transformation|GetVelocity)) 0.0)
            (CallFunction|Attack0)
            (goto _label)
            (else
              _))))
      (else
        (Variables|Default|SetisAttacking false)
        (if (Variables|Default|GetisDead)
          _
          (else
            (Utilities|FlowControl|Delay (Variables|Default|GetAttackDelay))))))
    (Variables|Default|SetisAttacking false)))

(event Custom|UpdateAnimation
  (CallFunction|Rotate)
  (if (Variables|Default|GetisDead)
    _
    (else
      (if (and (> (Math|Vector|VectorLength (Transformation|GetVelocity)) 0.0) (AI|Components|NavMovement|IsMovingonGround (Variables|Character|GetCharacterMovement)))
        (Variables|Default|SetAnimationState "NewEnumerator4")
        (else
          (Variables|Default|SetAnimationState "NewEnumerator0")))
      (if (Variables|Default|GetisAttacking)
        (Variables|Default|SetAnimationState "NewEnumerator5"))
      (CallFunction|CheckZone)))
  (bind _returnvalue (CallFunction|GetFlipbook (Variables|Default|GetAnimationState)))
  (Sprite|SetFlipbook (Variables|Default|GetSprite) _returnvalue))

(event Custom|DeadFinSprite
  (Variables|Default|SetAnimationState (Utilities|Select :Index (Variables|Default|GetDeadType) :NewEnumerator0 "NewEnumerator10" :NewEnumerator1 "NewEnumerator11")))

(event Custom|EnemyGo
  (AI|AIMoveTo (Class|CharacterMovementComponent|GetCharacterOwner (Variables|Character|GetCharacterMovement)) "0, 0, 0" (Game|GetPlayerController 0) 2e+02 true
    (:OnSuccess
      (CallFunction|OnAttacking)
      (Utilities|FlowControl|Delay 1.0))))

(event EventBeginPlay
  (|CallParentFunction)
  (bind _outactors (Actor|GetAllActorsOfClass "/Game/Blueprint/Characters/JapaniseBun/BP_Character_Bun.BP_Character_Bun_C"))
  (Variables|Default|SetPlayerChar (Utilities|Array|Get(acopy) _outactors))
  (Variables|Default|SetEnemy (Components|GetOwner (Variables|Default|GetCapsuleComponent))))

(event Collision|EventActorBeginOverlap
  (params (OtherActor :type Actor%20Object%20Reference))
  (|CallParentFunction OtherActor) ; This node is disabled and will not be called.\nDrag off pins to build functionality.
)

(event EventTick
  (params (DeltaSeconds :type Float%20%28single-precision%29))
  (|CallParentFunction DeltaSeconds)
  (CallFunction|UpdateAnimation))

(fn ConstructionScript
  (|CallParentFunction))

(fn Attack0
  (bind _returnvalue (Math|Random|RandomFloatinRange 1e+04 3e+04))
  (bind _multiplierdir (Variables|Default|GetmultiplierDir))
  (bind _returnvalue_2 (* _returnvalue 1.0))
  (if (not (Variables|Default|GetisDead))
    (bind _returnvalue_3 (Game|SpawnActorfromClass "/Game/Blueprint/Characters/Donut/BP_Dot.BP_Dot_C" (Math|Transform|MakeTransform (Transformation|GetSocketLocation (Variables|Default|GetSprite) "Socket_0") "0, 0, 0" "1.000000,1.000000,1.000000") "AlwaysSpawn" "MultiplyWithRoot" 0 0))
    (Variables|/Game/Blueprint/Characters/Donut/BP_Dot.BP_Dot_C|SetEnemy _returnvalue_3 (Variables|Default|GetEnemy))
    (CallFunction|GetDirMultiplyer)
    (bind _output_get (Variables|Default|SetDotImpulse (+ (Utilities|Select :Index (Variables|Default|GetActiveZone) :NewEnumerator0 (* (Math|Vector|MakeVector _multiplierdir 0.0 1.0) (Math|Vector|MakeVector _returnvalue_2 0.0 _returnvalue_2)) :NewEnumerator1 (* (Math|Vector|MakeVector _multiplierdir 0.0 1.0) (Math|Vector|MakeVector _returnvalue 0.0 _returnvalue)) :NewEnumerator2 (* (Math|Vector|MakeVector (Variables|Default|GetmultiplierDir) 0.0 1.0) (Math|Vector|MakeVector (Math|Random|RandomFloatinRange 7e+04 1e+05) 0.0 0.0))) (Transformation|GetVelocity))))
    (Physics|AddImpulse (Variables|/Game/Blueprint/Characters/Donut/BP_Dot.BP_Dot_C|GetSphere _returnvalue_3) _output_get "None" false)))

(fn GetFlipbook
  (params (Index :type E_AnimationState%20Enum :default "NewEnumerator0"))
  (return (Utilities|Select :Index Index :NewEnumerator0 (Variables|Default|GetIdle) :NewEnumerator1 0 :NewEnumerator2 0 :NewEnumerator3 0 :NewEnumerator4 (Variables|Default|GetWalk) :NewEnumerator5 (Variables|Default|GetAttacking) :NewEnumerator6 0 :NewEnumerator7 0 :NewEnumerator8 (Variables|Default|GetDead_01) :NewEnumerator9 (Variables|Default|GetDead_02) :NewEnumerator10 (Variables|Default|GetDead_01_static) :NewEnumerator11 (Variables|Default|GetDead_02_static))))

(fn CheckZone
  (if (not (Variables|Default|GetisDead))
    (Variables|Default|SetActiveZone "NewEnumerator0")
    (bind _asbp_character_bun (Utilities|Casting|CastToBP_Character_Bun (Game|GetPlayerCharacter 0)))
    (if (Collision|IsOverlappingActor (Variables|Default|GetCheck_far_zone) _asbp_character_bun :!class /Script/Engine.PrimitiveComponent)
      (Variables|Default|SetActiveZone "NewEnumerator1"))
    (if (Collision|IsOverlappingActor (Variables|Default|GetCheck_near_zone) _asbp_character_bun :!class /Script/Engine.PrimitiveComponent)
      (Variables|Default|SetActiveZone "NewEnumerator2")
      (return))))

(fn Dead
  (params (DeadType :type E_DeadType%20Enum :default "NewEnumerator0"))
  (bind _returnvalue (Components|GetOwner))
  (bind _returnvalue_2 (AI|GetAIController _returnvalue))
  (if (not (Variables|Default|GetisDead))
    (Variables|Default|SetisAttacking false)
    (Variables|Default|SetisDead true)
    (Variables|Default|SetAnimationState (Utilities|Select :Index DeadType :NewEnumerator0 "NewEnumerator8" :NewEnumerator1 "NewEnumerator9"))
    (AI|Logic|StopLogic (Variables|/Script/AIModule.AIController|GetBrainComponent _returnvalue_2) "")
    (Class|AIPerceptionComponent|SetSenseEnabled (Class|AIController|GetAIPerceptionComponent _returnvalue_2) "/Script/AIModule.AISense_Sight" false)
    (Physics|SetSimulatePhysics (Variables|Default|GetCapsuleComponent) false)
    (Physics|SetEnableGravity (Variables|Default|GetCapsuleComponent) false)
    (Collision|SetCollisionEnabled (Variables|Default|GetCapsuleComponent) "NoCollision")
    (Collision|SetCollisionEnabled (Variables|Default|GetDangerCheck) "NoCollision")
    (Utilities|Time|SetTimerbyEvent (EventDispatchers|CreateEvent :!event Custom|DeadFinSprite) (Utilities|Select :Index (Variables|Default|GetAnimationState) :NewEnumerator0 0.0 :NewEnumerator1 0.0 :NewEnumerator2 0.0 :NewEnumerator3 0.0 :NewEnumerator4 0.0 :NewEnumerator5 0.0 :NewEnumerator6 0.0 :NewEnumerator7 0.0 :NewEnumerator8 0.2 :NewEnumerator9 0.3 :NewEnumerator10 0.0 :NewEnumerator11 0.0))
    (return)))

(fn GetDirMultiplyer
  (if (<= (.x (- (Transformation|GetActorLocation (Variables|Default|GetPlayerChar)) (Transformation|GetSocketLocation (Variables|Default|GetSprite) "Socket_0"))) 0.0)
    (Variables|Default|SetmultiplierDir -1.0)
    (else
      (Variables|Default|SetmultiplierDir 1.0)))
  (return (Variables|Default|GetmultiplierDir)))

(fn Rotate
  (bind _returnvalue (Transformation|GetVelocity))
  (bind _sprite (Variables|Default|GetSprite))
  (if (not (Variables|Default|GetisDead))
    (if (> (.x _returnvalue) 0.0)
      (Transformation|SetWorldRotation _sprite "0.000000,180.000000,0.000000" false false)
      (Variables|Default|SetcurrentRotator "0.000000,180.000000,0.000000")
      (elif (< (.x _returnvalue) 0.0)
        (Transformation|SetWorldRotation _sprite "0, 0, 0" false false)
        (Variables|Default|SetcurrentRotator "0, 0, 0")
        (else
          (Transformation|SetWorldRotation _sprite (Variables|Default|GetcurrentRotator) false false))))))