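; BP_Dot is a short-lived physics-driven flipbook dot that splats on impact, ignoring hits with BP_Donut and other dots.
; On spawn it takes a random size and translucent sort priority, then pops in through a scale timeline.
; Tick aligns it to the sphere's velocity while alive.
; After impact, Tick stops physics, fixes rotation, sinks it, shows the hit flipbook and destroys it after a brief delay.
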(event OnComponentHit(Sphere)
  (params (HitComponent :type Primitive%20Component%20Object%20Reference) (OtherActor :type Actor%20Object%20Reference) (OtherComp :type Primitive%20Component%20Object%20Reference) (NormalImpulse :type Vector :default "0, 0, 0") (Hit :type Hit%20Result%20Structure%20%28by%20ref%29))
  (Utilities|Casting|CastToBP_Donut OtherActor
    (:CastFailed
      (Utilities|Casting|CastToBP_Dot OtherActor
        (:CastFailed
          (Variables|Default|SetisAlive false))))))

(event EventBeginPlay
  (Variables|Default|SetDotScale (Math|Random|RandomFloatinRange 2.0 4.0))
  (Rendering|SetTranslucentSortPriority (Variables|Default|GetPaperFlipbook) (Math|Random|RandomIntegerinRange 100 100000))
  (Components|Timeline|SetPlayRate (Variables|Default|GetScaleAnim) 8.0)
  (bind _newtrack_0 (Timeline|ScaleAnim PlayFromStart)
    (:Update
      (Transformation|SetWorldScale3D (Variables|Default|GetPaperFlipbook) (Math|Vector|MakeVector (* (Variables|Default|GetDotScale) _newtrack_0) (* (Variables|Default|GetDotScale) _newtrack_0) (* (Variables|Default|GetDotScale) _newtrack_0))))))

(event Collision|EventActorBeginOverlap
  (params (OtherActor :type Actor%20Object%20Reference)))

(event EventTick
  (params (DeltaSeconds :type Float%20%28single-precision%29))
  (if (Variables|Default|GetisAlive)
    (Transformation|SetWorldRotation (Variables|Default|GetScene) (Math|Rotator|MakeRotfromX (Transformation|GetComponentVelocity (Variables|Default|GetSphere))) false false)
    (else
      (Physics|SetSimulatePhysics (Variables|Default|GetSphere) false)
      (Transformation|SetWorldRotation (Variables|Default|GetScene) "270.000000,0.000000,0.000000" false false)
      (Transformation|SetWorldLocation (Variables|Default|GetScene) (+ (Transformation|GetWorldLocation (Variables|Default|GetScene)) "0.000000,0.000000,-2.000000") false false)
      (Sprite|SetFlipbook (Variables|Default|GetPaperFlipbook) "/Game/PaperAssets/Dot/Dot_v01__hit.Dot_v01__hit")
      (Utilities|FlowControl|Delay 0.2)
      (Actor|DestroyActor))))

(fn ConstructionScript)